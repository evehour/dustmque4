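; BpCamera is a camera director actor that controls which camera the first player controller views through.
; On BeginPlay it enables input for that controller and sets the view target to MainCamera.
; SwitchCamera flips a Select flag and blends the view to Camera1 or Camera2, with a different blend time for each.
; The event graph's only SwitchCamera call is unconnected, so this graph never triggers the toggle.
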(event `self.ReceiveBeginPlay`
  (bind _returnvalue (`GameplayStatics.GetPlayerController` 0))
  (`self.EnableInput` _returnvalue)
  (`PlayerController.SetViewTargetWithBlend` _returnvalue (`self.MainCamera`) 0.0 "VTBlend_Linear" 0.0 false))

(event `InputAction|Jump`
  (params (Key :type "Key Structure")))

(fn `SwitchCamera`
  (bind _returnvalue (`GameplayStatics.GetPlayerController` 0))
  (bind _select (`self.Select`))
  (set `self.Select` (not _select))
  (if _select
    (`PlayerController.SetViewTargetWithBlend` _returnvalue (`self.Camera1`) 2.0 "VTBlend_Linear" 0.0 false)
    (else
      (`PlayerController.SetViewTargetWithBlend` _returnvalue (`self.Camera2`) 1.0 "VTBlend_Linear" 0.0 false))))

(fn `UserConstructionScript`)