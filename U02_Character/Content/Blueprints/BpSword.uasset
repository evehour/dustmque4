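; BpSword is a player-controlled sword character that moves along world axes, jumps and attacks with montages.
; An Attack flag blocks movement, jumping and repeat attacks until AttackEnd clears it.
; A Capsule hitbox starts with collision off, is toggled by the OnStartCollision and OnEndCollision events, and destroys any other actor it begins overlapping.
; Landing stops the jump montage.
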(event `InputAxis|MoveForward`
  (params (AxisValue :type "Float (single-precision)"))
  (`self.Moving` AxisValue (1.0 0.0 0.0)))

(event `InputAxis|MoveRight`
  (params (AxisValue :type "Float (single-precision)"))
  (`self.Moving` AxisValue (0.0 10.0 0.0)))

(event `self.ReceiveBeginPlay`
  (`PrimitiveComponent.SetCollisionEnabled` (`self.Capsule`) "NoCollision"))

(event `InputAction|Jump`
  (params (Key :type "Key Structure"))
  (:`Pressed`
    (`self.Jumping`))
  (:`Released`
    (`self.StopJumping`)))

(event `self.OnLanded`
  (params (Hit :type "HitResult Structure (by ref)"))
  (`self.StopAnimMontage` "/Game/Montages/BpMonSwordJump.BpMonSwordJump"))

(event `InputAction|Attack`
  (params (Key :type "Key Structure"))
  (:`Pressed`
    (`self.Attacking`)))

(event `AttackEnd`
  (`self.Attacked`))

(event `self.Capsule.OnComponentBeginOverlap`
  (params (OverlappedComponent :type "PrimitiveComponent Object Reference") (OtherActor :type "Actor Object Reference") (OtherComp :type "PrimitiveComponent Object Reference") (OtherBodyIndex :type Integer) (bFromSweep :type Boolean) (SweepResult :type "HitResult Structure (by ref)"))
  ;[1 1 1] Collision
  (if (not (== self OtherActor))
    (`self.K2_DestroyActor` OtherActor)))

(event `OnStartCollision`
  ;[1 1 1] Collision
  (`PrimitiveComponent.SetCollisionEnabled` (`self.Capsule`) "QueryAndPhysics"))

(event `OnEndCollision`
  ;[1 1 1] Collision
  (`PrimitiveComponent.SetCollisionEnabled` (`self.Capsule`) "NoCollision"))

(fn `Attacked`
  (set `self.bAttack` false))

(fn `Attacking`
  (if (not (`self.bAttack`))
    (set `self.bAttack` true)
    (`self.PlayAnimMontage` "/Game/Montages/BpMonSwordAttack.BpMonSwordAttack")))

(fn `Jumping`
  (if (`NavMovementComponent.IsFalling` (`self.CharacterMovement`))
    _
    (elif (not (`self.bAttack`))
      (`self.Jump`)
      (`self.PlayAnimMontage` "/Game/Montages/BpMonSwordJump.BpMonSwordJump"))))

(fn `Moving`
  (params (Value :type "Float (double-precision)") (Direction :type "Vector Structure"))
  (if (not (`self.bAttack`))
    (`self.AddMovementInput` Direction Value)))

(fn `UserConstructionScript`)